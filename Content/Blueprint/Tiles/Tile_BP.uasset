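; Tile Blueprint that scatters random collectables over itself when play begins and removes them when it is destroyed.
; On BeginPlay each spawn point gets a coin-flip chance to spawn an actor of a random class from the collectable type list, stored in an array.
; On Destroyed it destroys every still-valid actor in that array, so collectables do not outlive their tile.
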(event `self.ReceiveBeginPlay`
  (for _array_element (`self.SpawnPoints`)
    (if (`KismetMathLibrary.RandomBool`)
      (bind _returnvalue (`|SpawnActorFromClass` (`self.GetRandomCollectableType`) (`SceneComponent.K2_GetComponentToWorld` _array_element) "Undefined" "OverrideRootScale" null null))
      (`KismetArrayLibrary.Array_Add` (`self.Collectables`) _returnvalue))))

(event `self.ReceiveDestroyed`
  (for _array_element (`self.Collectables`)
    (if (`KismetSystemLibrary.IsValid` _array_element)
      (`self.K2_DestroyActor` _array_element))))

(fn `GetRandomCollectableType`
  (returns (Output :type "Actor Class Reference"))
  (bind _spawncollectabletypes (`self.SpawnCollectableTypes`))
  (return (`|GetArrayItem` _spawncollectabletypes (`KismetMathLibrary.RandomInteger` (`KismetArrayLibrary.Array_Length` _spawncollectabletypes)))))

(fn `UserConstructionScript`)