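; UnstoppableMan_BP is a player Blueprint that gives the character a timed movement speed boost.
; The SpeedBoost event adds Power to max walk speed through SpeedBoostStart only when no boost is active, guarded by the Boosted flag.
; A retriggerable delay lets repeat calls restart the timer without stacking speed.
; When it expires, SpeedBoostStop subtracts the most recently stored Power and the flag clears.
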(event `Event SpeedBoost`
  (params (Power :type "Float (double-precision)") (Duration :type "Float (double-precision)"))
  (set `self.Power` Power)
  (set `self.Duration` Duration)
  (if (not (`self.Boosted`))
    (`self.SpeedBoostStart` (`self.Power`))
    (set `self.Boosted` true))
  (`KismetSystemLibrary.RetriggerableDelay` (`self.Duration`))
  (`self.SpeedBoostStop` (`self.Power`))
  (set `self.Boosted` false))

(fn `SpeedBoostStart`
  (params (Power :type "Float (double-precision)"))
  (set `CharacterMovementComponent.MaxWalkSpeed` (+ (`CharacterMovementComponent.MaxWalkSpeed` (`self.CharacterMovement`)) Power) (`self.CharacterMovement`))
  (`KismetSystemLibrary.PrintString` "Start"))

(fn `SpeedBoostStop`
  (params (Power :type "Float (double-precision)"))
  (set `CharacterMovementComponent.MaxWalkSpeed` (- (`CharacterMovementComponent.MaxWalkSpeed` (`self.CharacterMovement`)) Power) (`self.CharacterMovement`))
  (`KismetSystemLibrary.PrintString` "End"))

(fn `UserConstructionScript`)