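; SpeedBooster_BP is a collectable that temporarily boosts the walk speed of the UnstoppableMan_BP character that overlaps its Collider.
; On overlap it adds Power to MaxWalkSpeed, hides itself, waits five seconds, then subtracts Power and destroys itself.
; Collision stays active while hidden, so a repeat overlap during the delay adds Power again, while the pending delay subtracts it only once.
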(event `self.Collider.OnComponentBeginOverlap`
  (params (OverlappedComponent :type "PrimitiveComponent Object Reference") (OtherActor :type "Actor Object Reference") (OtherComp :type "PrimitiveComponent Object Reference") (OtherBodyIndex :type Integer) (bFromSweep :type Boolean) (SweepResult :type "HitResult Structure (by ref)"))
  (bind _charactermovement (`Character.CharacterMovement` (`self.UnstoppableMan`)))
  (bind _asunstoppable_man_bp (cast `/Game/Blueprint/Player/UnstoppableMan_BP` OtherActor))
  (bind _output_get (set `self.UnstoppableMan` _asunstoppable_man_bp))
  (bind _charactermovement_2 (`Character.CharacterMovement` _output_get))
  (set `CharacterMovementComponent.MaxWalkSpeed` (+ (`CharacterMovementComponent.MaxWalkSpeed` _charactermovement_2) (`self.Power`)) _charactermovement_2)
  (`self.SetActorHiddenInGame` true)
  (`KismetSystemLibrary.Delay` 5.0)
  (set `CharacterMovementComponent.MaxWalkSpeed` (- (`CharacterMovementComponent.MaxWalkSpeed` _charactermovement) (`self.Power`)) _charactermovement)
  (`self.K2_DestroyActor`))

(fn `UserConstructionScript`)