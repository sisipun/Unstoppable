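; Base game mode that manages a rolling chain of level tiles, adding one at the end and removing one from the start on each SpawnTile event.
; SpawnNewTile spawns a Tile_BP at LastTile's AttachPoint transform and stores it as the new LastTile.
; DestroyFirstTile destroys FirstTile, then InitFirstTile selects the next from GetAllActorsOfClass, relying on array order.
; InitLastTile similarly takes the array's last entry but is not called here.
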(event `self.SpawnTile`
  (`self.SpawnNewTile`)
  (`self.DestroyFirstTile`))

(fn `DestroyFirstTile`
  (`self.K2_DestroyActor` (`self.FirstTile`))
  (`self.InitFirstTile`))

(fn `InitFirstTile`
  (bind _outactors (`GameplayStatics.GetAllActorsOfClass` "/Script/Unstoppable.Tile"))
  (set `self.FirstTile` (`|GetArrayItem` _outactors)))

(fn `InitLastTile`
  (bind _outactors (`GameplayStatics.GetAllActorsOfClass` "/Script/Unstoppable.Tile"))
  (set `self.LastTile` (`|GetArrayItem` _outactors (`KismetArrayLibrary.Array_LastIndex` _outactors))))

(fn `SpawnNewTile`
  (bind _returnvalue (`|SpawnActorFromClass` "/Game/Blueprint/Tiles/Tile_BP.Tile_BP_C" (`SceneComponent.K2_GetComponentToWorld` (`Tile.AttachPoint` (`self.LastTile`))) "Undefined" "OverrideRootScale" null null))
  (set `self.LastTile` _returnvalue))

(fn `UserConstructionScript`)